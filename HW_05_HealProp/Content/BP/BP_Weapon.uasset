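; BP_Weapon is an automatic firearm Blueprint with magazine and reserve ammo, using a SKAR4 mesh.
; While the Fire input is held, a Delay-paced loop spawns an actor and muzzle flash at the mesh's ammo socket, decrementing CurrentAmmo until empty or released.
; The Reload event refills the magazine from RemainAmmo, capping the transfer at what is left in reserve.
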(event `InputAction|Fire`
  (params (Key :type "Key Structure"))
  (bind _sk_ar4 (`self.SK_AR4`))
  ;[1 1 1] Fire
  (:`Pressed`
    (set `self.Fireing` true)
    (if (and (> (`self.CurrentAmmo`) 0) (`self.Fireing`)) :!label _label
      (`|SpawnActorFromClass` "/Game/BP/BP_Ammo.BP_Ammo_C" (`SceneComponent.GetSocketTransform` (`self.SK_AR4`) "Ammo Socket" "RTS_World") "Undefined" "OverrideRootScale" null null)
      (`GameplayStatics.SpawnEmitterAtLocation` "/Game/InfinityBladeEffects/Effects/FX_Monsters/FX_Monster_Gruntling/Master/P_BackPack_MuzzleFlash.P_BackPack_MuzzleFlash" (`SceneComponent.GetSocketLocation` _sk_ar4 "Ammo Socket") (`SceneComponent.GetSocketRotation` _sk_ar4 "Ammo Socket") (0.08 0.08 0.08))
      (set `self.CurrentAmmo` (- (`self.CurrentAmmo`) 1))
      (`KismetSystemLibrary.Delay` (`self.FireDuration`))
      (goto _label)))
  (:`Released`
    (set `self.Fireing` false)))

(event `Reload`
  ;[1 1 1] Count how much need to restore
  (set `self.RestoredAmmo` (- (`self.MagazineSize`) (`self.CurrentAmmo`)))
  ;[1 1 1] Is it RemainAmmo>=Restored ?
  (if (not (>= (`self.RemainAmmo`) (`self.RestoredAmmo`)))
    ;[1 1 1] Remain < Restored
    (set `self.RestoredAmmo` (`self.RemainAmmo`)))
  ;[1 1 1] Update CurrentAmmo and RemainAmmo
  (set `self.CurrentAmmo` (+ (`self.CurrentAmmo`) (`self.RestoredAmmo`)))
  (set `self.RemainAmmo` (- (`self.RemainAmmo`) (`self.RestoredAmmo`))))

(fn `UserConstructionScript`)